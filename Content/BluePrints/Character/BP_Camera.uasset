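; BP_Camera is a camera Blueprint that performs a timed vertical pan toward the PlayerStartZ height.
; A short delay after BeginPlay sets StartPan, letting Tick ease the actor's Z with FInterpTo while keeping X and Y.
; It feeds world location into SetActorRelativeLocation.
; A Delay inside Tick later clears StartPan and sets FinishedPanning, ending the pan on time rather than on arrival.
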(event EventBeginPlay
  (Utilities|FlowControl|Delay 2.0)
  (Variables|Default|SetStartPan true))

(event Collision|EventActorBeginOverlap
  (params (OtherActor :type Actor%20Object%20Reference)))

(event EventTick
  (params (DeltaSeconds :type Float%20%28single-precision%29))
  (bind _self self)
  (bind _returnvalue (Transformation|GetActorLocation _self))
  (if (Variables|Default|GetStartPan)
    (Transformation|SetActorRelativeLocation (Math|Vector|MakeVector (.x _returnvalue) (.y _returnvalue) (Math|Interpolation|FInterpTo (.z _returnvalue) (Variables|Default|GetPlayerStartZ) (Utilities|Time|GetWorldDeltaSeconds) 0.6)))
    (Utilities|FlowControl|Delay 8.0)
    (Variables|Default|SetStartPan false)
    (Variables|Default|SetFinishedPanning true)))

(fn ConstructionScript)