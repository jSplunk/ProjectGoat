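; BP_Death is a death trigger that respawns the player by returning BP_MainCharacter to its StartingLocation on overlap.
; It also moves BP_Camera to a hardcoded height, feeding its current world X and Y into a relative-location set.
; The reset runs only while MoveCamera's HasOverlapped flag is false, and end overlap clears that flag.
; The overlapping actor is never checked, so any overlap resets player 0.
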(event EventBeginPlay)

(event Collision|EventActorBeginOverlap
  (params (OtherActor :type Actor%20Object%20Reference))
  (if (not (Variables|/Game/BluePrints/Character/BP_MoveCamera.BP_MoveCamera_C|GetHasOverlapped (Variables|Default|GetMoveCamera)))
    (bind _asbp_main_character (Utilities|Casting|CastToBP_MainCharacter (Game|GetPlayerCharacter 0)))
    (Transformation|SetActorLocation _asbp_main_character (Variables|/Game/BluePrints/Character/BP_MainCharacter.BP_MainCharacter_C|GetStartingLocation _asbp_main_character) false false)
    (bind _returnvalue (Actor|GetActorOfClass "/Game/BluePrints/Character/BP_Camera.BP_Camera_C"))
    (Transformation|SetActorRelativeLocation _returnvalue (Math|Vector|MakeVector (.x (Transformation|GetActorLocation _returnvalue)) (.y (Transformation|GetActorLocation _returnvalue)) 4.26e+03))))

(event EventTick
  (params (DeltaSeconds :type Float%20%28single-precision%29)))

(event Collision|EventActorEndOverlap
  (params (OtherActor :type Actor%20Object%20Reference))
  (Variables|/Game/BluePrints/Character/BP_MoveCamera.BP_MoveCamera_C|SetHasOverlapped (Variables|Default|GetMoveCamera) false))

(fn ConstructionScript)