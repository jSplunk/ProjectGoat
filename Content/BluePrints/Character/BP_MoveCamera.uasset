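; BP_MoveCamera is an overlap-triggered actor that pans the level's BP_Camera vertically toward NewCameraLocation.
; Any actor overlap sets HasOverlapped, finds the camera and starts panning.
; Tick eases only the camera's Z with VInterpTo, feeding its world location into SetActorRelativeLocation.
; Panning stops when Z exactly equals the target, or half a second after an overlap ends.
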(event EventBeginPlay)

(event Collision|EventActorBeginOverlap
  (params (OtherActor :type Actor%20Object%20Reference))
  (Variables|Default|SetHasOverlapped true)
  (Variables|Default|SetStartPanning true)
  (bind _returnvalue (Actor|GetActorOfClass "/Game/BluePrints/Character/BP_Camera.BP_Camera_C"))
  (Variables|Default|SetCameraActor _returnvalue))

(event EventTick
  (params (DeltaSeconds :type Float%20%28single-precision%29))
  (bind _cameraactor (Variables|Default|GetCameraActor))
  (bind _returnvalue (Transformation|GetActorLocation _cameraactor))
  (if (Variables|Default|GetStartPanning)
    (Transformation|SetActorRelativeLocation (Variables|Default|GetCameraActor) (Math|Interpolation|VInterpTo (Transformation|GetActorLocation (Variables|Default|GetCameraActor)) (Math|Vector|MakeVector (.x _returnvalue) (.y _returnvalue) (Variables|Default|GetNewCameraLocation)) (Utilities|Time|GetWorldDeltaSeconds) 2.0))
    (if (== (Variables|Default|GetNewCameraLocation) (.z (Transformation|GetActorLocation (Variables|Default|GetCameraActor))))
      (Variables|Default|SetStartPanning false))))

(event Collision|EventActorEndOverlap
  (params (OtherActor :type Actor%20Object%20Reference))
  (Utilities|FlowControl|Delay 0.5)
  (Variables|Default|SetStartPanning false))

(fn ConstructionScript)