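; Player character for a side-scrolling 2D platformer, moving along the Y axis with a charged high jump and a mid-air double jump.
; Holding high jump locks movement and builds jump power, then launches in the facing direction.
; The double jump works once per airtime while falling, deriving Z velocity from fall speed.
; Tick flips the sprite by velocity and enables input once BP_Camera finishes panning, while jump events drive animation nodes.
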(event Custom|StartMoving
  (bind _returnvalue (Game|GetPlayerController 0))
  (bind _returnvalue_2 (PlayerController|LocalPlayerSubsystems|GetEnhancedInputLocalPlayerSubsystem _returnvalue))
  (if (Variables|/Game/BluePrints/Character/BP_Camera.BP_Camera_C|GetFinishedPanning (Variables|Default|GetCamera))
    (Utilities|FlowControl|DoOnce false
      (:Completed
        (Utilities|IsValid _returnvalue_2
          (:Is%20Valid
            (Input|AddMappingContext _returnvalue_2 "/Game/BluePrints/IA_MainCharacter.IA_MainCharacter" 0 "(bIgnoreAllPressedKeysUntilRelease=True,bForceImmediately=False)")))))))

(event Custom|GetCamera
  (if (not (Utilities|IsValid (Variables|Default|GetCamera)))
    (bind _returnvalue (Actor|GetActorOfClass "/Game/BluePrints/Character/BP_Camera.BP_Camera_C"))
    (Variables|Default|SetCamera _returnvalue)))

(event Custom|Update%20Player%20Rotation
  (Math|Float|CompareFloat (.y (Variables|/Script/Engine.MovementComponent|GetVelocity (Variables|Character|GetCharacterMovement))) 0.0
    (:>
      (Transformation|SetRelativeRotation (Variables|Default|GetSprite) "0.000000,0.000000,0.000000" false false)
      (Variables|Default|SetFacingLeft false)
      (Variables|Default|SetFacingRight true))
    (:<
      (Transformation|SetRelativeRotation (Variables|Default|GetSprite) "0.000000,-180.000000,0.000000" false false)
      (Variables|Default|SetFacingLeft true)
      (Variables|Default|SetFacingRight false))))

(event Input|EnhancedActionEvents|EnhancedInputActionIA_MoveRight
  (params (ActionValue :type Float%20%28double-precision%29) (ElapsedSeconds :type Float%20%28double-precision%29) (TriggeredSeconds :type Float%20%28double-precision%29) (InputAction :type Input%20Action%20Object%20Reference :default "/Game/BluePrints/IA_MoveRight.IA_MoveRight"))
  (:Triggered
    (if (not (Variables|Default|GetMovementLocked))
      (Pawn|Input|AddMovementInput "0.000000,1.000000,0.000000" ActionValue false))))

(event Input|EnhancedActionEvents|EnhancedInputActionIA_Jump
  (params (ActionValue :type Boolean) (ElapsedSeconds :type Float%20%28double-precision%29) (TriggeredSeconds :type Float%20%28double-precision%29) (InputAction :type Input%20Action%20Object%20Reference :default "/Game/BluePrints/IA_Jump.IA_Jump"))
  (bind _self self)
  (bind _charactermovement (Variables|Character|GetCharacterMovement _self))
  (:Triggered
    (if (and (Variables|Default|GetCanStillJump) (not (Variables|Default|GetDoubleJump)))
      (if (< (.z (Variables|/Script/Engine.MovementComponent|GetVelocity _charactermovement)) 0.0)
        (bind _result (Math|Float|NegateFloat (.z (Variables|/Script/Engine.MovementComponent|GetVelocity _charactermovement)))
          (:%20%20
            (Variables|/Script/Engine.MovementComponent|SetVelocity _charactermovement (Math|Vector|MakeVector (.x (Variables|/Script/Engine.MovementComponent|GetVelocity _charactermovement)) (.y (Variables|/Script/Engine.MovementComponent|GetVelocity _charactermovement)) (/ _result 2.0)))
            (Variables|Default|SetDoubleJump true)))))))

(event Input|EnhancedActionEvents|EnhancedInputActionIA_JumpHigh
  (params (ActionValue :type Float%20%28double-precision%29) (ElapsedSeconds :type Float%20%28double-precision%29) (TriggeredSeconds :type Float%20%28double-precision%29) (InputAction :type Input%20Action%20Object%20Reference :default "/Game/BluePrints/IA_JumpHigh.IA_JumpHigh"))
  (bind _self self)
  (bind _charactermovement (Variables|Character|GetCharacterMovement))
  (bind _charactermovement_2 (Variables|Character|GetCharacterMovement _self))
  (:Triggered
    (if (Variables|Default|GetCanStillJump)
      (Variables|/Script/Engine.CharacterMovementComponent|SetJumpZVelocity _charactermovement_2 (* (Variables|Default|GetJumpVelMultiplier) 1e+02))
      (if (Variables|Default|GetFacingLeft)
        (Variables|/Script/Engine.MovementComponent|SetVelocity _charactermovement (Math|Vector|MakeVector (.x (Variables|/Script/Engine.MovementComponent|GetVelocity _charactermovement)) -4e+02 (.z (Variables|/Script/Engine.MovementComponent|GetVelocity _charactermovement))))
        (else
          (Variables|/Script/Engine.MovementComponent|SetVelocity _charactermovement (Math|Vector|MakeVector (.x (Variables|/Script/Engine.MovementComponent|GetVelocity _charactermovement)) 4e+02 (.z (Variables|/Script/Engine.MovementComponent|GetVelocity _charactermovement))))))
      (Character|Jump)))
  (:Started
    (if (== (.z (Variables|/Script/Engine.MovementComponent|GetVelocity (Variables|Character|GetCharacterMovement))) 0.0)
      (Class|PaperZDAnimInstance|JumptoNode (Variables|/Script/PaperZD.PaperZDAnimationComponent|GetAnimInstance (Variables|Default|GetAnimationComponent)) "jump_prepare" "None")
      (Variables|Default|SetMovementLocked true)))
  (:Ongoing
    (if (< (Variables|Default|GetJumpVelMultiplier) 1e+01)
      (bind _output_get (Variables|Default|SetJumpVelMultiplier (+ (Variables|Default|GetJumpVelMultiplier) 0.4)))))
  (:Completed
    (Variables|/Script/Engine.CharacterMovementComponent|SetJumpZVelocity _charactermovement_2 (Variables|Default|GetInitialJumpZ))
    (Character|StopJumping)
    (Variables|Default|SetJumpVelMultiplier 0.0)
    (Variables|Default|SetMovementLocked false)))

(event Input|EnhancedActionEvents|EnhancedInputActionIA_MoveLeft
  (params (ActionValue :type Float%20%28double-precision%29) (ElapsedSeconds :type Float%20%28double-precision%29) (TriggeredSeconds :type Float%20%28double-precision%29) (InputAction :type Input%20Action%20Object%20Reference :default "/Game/BluePrints/IA_MoveLeft.IA_MoveLeft"))
  (:Triggered
    (if (not (Variables|Default|GetMovementLocked))
      (Pawn|Input|AddMovementInput "0.000000,-1.000000,0.000000" ActionValue false))))

(event EventBeginPlay
  (Variables|Default|SetInitialJumpZ (Variables|/Script/Engine.CharacterMovementComponent|GetJumpZVelocity (Variables|Character|GetCharacterMovement self)))
  (Variables|Default|SetStartingLocation (Transformation|GetActorLocation self)))

(event EventOnJumped
  (bind _asbp_player_animation (Utilities|Casting|CastToBP_PlayerAnimation (Variables|/Script/PaperZD.PaperZDAnimationComponent|GetAnimInstance (Variables|Default|GetAnimationComponent))))
  (Variables|/Game/BluePrints/Character/BP_PlayerAnimation.BP_PlayerAnimation_C|SetDonePrepare _asbp_player_animation false)
  (Class|PaperZDAnimInstance|JumptoNode _asbp_player_animation "airborne" "None")
  (Variables|Default|SetMovementLocked false))

(event EventOnWalkingOffLedge
  (params (PreviousFloorImpactNormal :type Vector%20%28by%20ref%29 :default "0, 0, 0") (PreviousFloorContactNormal :type Vector%20%28by%20ref%29 :default "0, 0, 0") (PreviousLocation :type Vector%20%28by%20ref%29 :default "0, 0, 0") (TimeDelta :type Float%20%28single-precision%29))
  (bind _asbp_player_animation (Utilities|Casting|CastToBP_PlayerAnimation (Variables|/Script/PaperZD.PaperZDAnimationComponent|GetAnimInstance (Variables|Default|GetAnimationComponent))))
  (Variables|/Game/BluePrints/Character/BP_PlayerAnimation.BP_PlayerAnimation_C|SetDonePrepare _asbp_player_animation false)
  (Class|PaperZDAnimInstance|JumptoNode _asbp_player_animation "airborne" "None")
  (Variables|Default|SetMovementLocked false))

(event EventTick
  (params (DeltaSeconds :type Float%20%28single-precision%29))
  (CallFunction|UpdatePlayerRotation)
  (CallFunction|GetCamera)
  (CallFunction|StartMoving)
  (if (AI|Components|NavMovement|IsMovingonGround (Variables|Character|GetCharacterMovement))
    (Utilities|FlowControl|DoOnce false :!label _label
      (:Completed
        (Variables|Default|SetDoubleJump false)))
    (else
      (goto _label Reset))))

(fn ConstructionScript)